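; BP_EnemySpawner periodically spawns BP_BaseEnemy actors across the map while the enemy population is low.
; A looping timer started on BeginPlay calls SpawnEnemy, which checks the CurrentEnemies count in GS_FastFPS against a cap.
; Each spawn lands at a random navigable point within a large radius of the world origin, using the game state's RecastNavmesh reference rather than the spawner's own location.
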(event `self.ReceiveBeginPlay`
  (`KismetSystemLibrary.K2_SetTimer` null "SpawnEnemy" 5.0 true))

(event `SpawnEnemy`
  (bind _asgs_fast_fps (cast `/Game/V2/GameMode/GS_FastFPS` (`GameplayStatics.GetGameState`)))
  (if (< (`KismetArrayLibrary.Array_Length` (`/Game/V2/GameMode/GS_FastFPS.CurrentEnemies` _asgs_fast_fps)) 10)
    ;[1 1 1] Spawn Enemy
    (bind _asgs_fast_fps_2 (cast `/Game/V2/GameMode/GS_FastFPS` (`GameplayStatics.GetGameState`)))
    (`|SpawnActorFromClass` "/Game/V2/Enemy/BP_BaseEnemy.BP_BaseEnemy_C" (`KismetMathLibrary.MakeTransform` (`NavigationSystemV1.K2_GetRandomLocationInNavigableRadius` (`KismetMathLibrary.MakeVector` 0.0) 5000.0 (`/Game/V2/GameMode/GS_FastFPS.RecastNavmesh` _asgs_fast_fps_2) null)) "Undefined" "OverrideRootScale" null null)))

(fn `UserConstructionScript`)