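; Base enemy Blueprint that starts chasing the player once the player character is within its detection volume.
; On BeginPlay it checks DetectionRage for an already overlapping C_PlayerCharacter, and later begin-overlap events catch one entering.
; Both paths cast the controller to AI_Controller and call StartChasingPlayer, leaving the chase itself to the controller.
; Nothing here stops the chase when the player leaves the volume.
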(event `self.ReceiveBeginPlay`
  ;[1 1 1] Chase Player when in range at Begin Play
  (if (> (`KismetArrayLibrary.Array_Length` (`PrimitiveComponent.GetOverlappingActors` (`self.DetectionRage`) "/Game/V2/Player/C_PlayerCharacter.C_PlayerCharacter_C")) 0)
    (`/Game/V2/Enemy/AI_Controller.StartChasingPlayer` (cast `/Game/V2/Enemy/AI_Controller` (`self.GetController`) :!pure true))))

(event `self.DetectionRage.OnComponentBeginOverlap`
  (params (OverlappedComponent :type "PrimitiveComponent Object Reference") (OtherActor :type "Actor Object Reference") (OtherComp :type "PrimitiveComponent Object Reference") (OtherBodyIndex :type Integer) (bFromSweep :type Boolean) (SweepResult :type "HitResult Structure (by ref)"))
  ;[1 1 1] Chase Player when in range
  (cast `/Game/V2/Player/C_PlayerCharacter` OtherActor)
  (`/Game/V2/Enemy/AI_Controller.StartChasingPlayer` (cast `/Game/V2/Enemy/AI_Controller` (`self.GetController`) :!pure true)))

(fn `UserConstructionScript`)