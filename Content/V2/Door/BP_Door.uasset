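; BP_Door is a kickable door that becomes a physics projectile able to hurt enemies.
; An overlap trigger binds the player's OnKick event, which launches the mesh along the player's forward vector, plays a sound, calls OnDoorKicked and destroys Box.
; A fast-moving door toggles capsule physics on overlapped enemies.
; Collision hits damage an enemy once and play throttled, speed-gated impact sounds.
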(event `self.PlayerInteraction.OnComponentBeginOverlap`
  (params (OverlappedComponent :type "PrimitiveComponent Object Reference") (OtherActor :type "Actor Object Reference") (OtherComp :type "PrimitiveComponent Object Reference") (OtherBodyIndex :type Integer) (bFromSweep :type Boolean) (SweepResult :type "HitResult Structure (by ref)"))
  (bind _asc_player_character (cast `/Game/V2/Player/C_PlayerCharacter` OtherActor)
    (:`then`
      (add `/Game/V2/Player/C_PlayerCharacter.OnKick` _asc_player_character (delegate `OnKick_Event_0`)))
    (:`CastFailed`
      (bind _asbp_base_enemy (cast `/Game/V2/Enemy/BP_BaseEnemy` OtherActor))
      (bind _returnvalue (`PrimitiveComponent.GetPhysicsLinearVelocity` (`self.StaticMesh`) "None"))
      (if (>= (`KismetMathLibrary.VSize` _returnvalue) 1500.0)
        (`/Game/V2/Enemy/BP_BaseEnemy.ToggleCapsulePhysics` _asbp_base_enemy 2.0)))))

(event `OnKick_Event_0`
  (params (Player :type "/Game/V2/Player/C_PlayerCharacter Object Reference"))
  (bind _staticmesh (`self.StaticMesh`))
  (`PrimitiveComponent.SetSimulatePhysics` _staticmesh true)
  (`PrimitiveComponent.SetPhysicsLinearVelocity` _staticmesh (* (`self.GetActorForwardVector` Player) 2000.0) false "None")
  (`GameplayStatics.PlaySoundAtLocation` "/Game/SFX/160213__qubodup__kicking-forcing-breaking-wooden-door.160213__qubodup__kicking-forcing-breaking-wooden-door" (`self.K2_GetActorLocation`) (struct) 2.0 1.0 0.1 null null null)
  (`self.OnDoorKicked`)
  (bind _box (`self.Box`)
    (:`then`
      (`ActorComponent.K2_DestroyComponent` _box))
    (:`else`)))

(event `self.PlayerInteraction.OnComponentEndOverlap`
  (params (OverlappedComponent :type "PrimitiveComponent Object Reference") (OtherActor :type "Actor Object Reference") (OtherComp :type "PrimitiveComponent Object Reference") (OtherBodyIndex :type Integer))
  (bind _asc_player_character (cast `/Game/V2/Player/C_PlayerCharacter` OtherActor))
  (remove `/Game/V2/Player/C_PlayerCharacter.OnKick` _asc_player_character (delegate `OnKick_Event_0`)))

(event `self.Collision.OnComponentHit`
  (params (HitComponent :type "PrimitiveComponent Object Reference") (OtherActor :type "Actor Object Reference") (OtherComp :type "PrimitiveComponent Object Reference") (NormalImpulse :type "Vector Structure") (Hit :type "HitResult Structure (by ref)"))
  (`|ExecutionSequence`
    (:`then_0`
      (bind _asbp_base_enemy (cast `/Game/V2/Enemy/BP_BaseEnemy` OtherActor))
      (`/Engine/EditorBlueprintResources/StandardMacros.DoOnce` false
        (:`Completed`
          (`GameplayStatics.ApplyDamage` _asbp_base_enemy 100.0))))
    (:`then_1`
      (`/Engine/EditorBlueprintResources/StandardMacros.DoOnce` false :!label _label
        (:`Completed`
          (bind _returnvalue (`PrimitiveComponent.GetPhysicsLinearVelocity` (`self.StaticMesh`) "None"))
          (if (>= (`KismetMathLibrary.VSize` _returnvalue) 300.0)
            (`GameplayStatics.PlaySoundAtLocation` "/Game/V2/Door/SC_DoorHit.SC_DoorHit" (`self.K2_GetActorLocation`) (struct) 2.0 1.0 0.0 null null null)
            (`KismetSystemLibrary.Delay` 0.2)
            (goto _label :!via `Reset`)))))))

(fn `UserConstructionScript`)